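; Road tile for an endless runner that chains the track as the player advances.
; When the character overlaps its Box, it has ThirdPersonGameMode spawn another tile, adds multiplier-scaled score, nudges clamped walk speed up, then destroys itself after a delay.
; BeginPlay stores and prints the X positions of four line markers.
; RandomSpawn, a draft chance-based obstacle spawner for Line1, is not currently called.
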(event OnComponentBeginOverlap(Box)
  (params (OverlappedComponent :type Primitive%20Component%20Object%20Reference) (OtherActor :type Actor%20Object%20Reference) (OtherComp :type Primitive%20Component%20Object%20Reference) (OtherBodyIndex :type Integer) (bFromSweep :type Boolean) (SweepResult :type Hit%20Result%20Structure%20%28by%20ref%29))
  ;[1 1 1] Cast Road
  (Utilities|Casting|CastToThirdPersonCharacter OtherActor)
  (bind _asthird_person_game_mode (Utilities|Casting|CastToThirdPersonGameMode (Game|GetGameMode)))
  (Default|SpawnTile _asthird_person_game_mode)
  ;[1 1 1] Score
  (bind _asthird_person_game_mode_2 (Utilities|Casting|CastToThirdPersonGameMode (Game|GetGameMode)))
  (bind _output_get (Variables|/Game/ThirdPersonBP/Blueprints/ThirdPersonGameMode.ThirdPersonGameMode_C|SetCurrentpoint _asthird_person_game_mode_2 (+ (* 1 (Variables|/Game/ThirdPersonBP/Blueprints/ThirdPersonGameMode.ThirdPersonGameMode_C|GetPointMultiplayer _asthird_person_game_mode_2)) (Variables|/Game/ThirdPersonBP/Blueprints/ThirdPersonGameMode.ThirdPersonGameMode_C|GetCurrentpoint _asthird_person_game_mode_2))))
  ;[1 1 1] ПРоверка
  (Development|PrintString (Utilities|String|ToString(Integer) _output_get))
  ;[1 1 1] Добавление к скорости 1.01 при пересечении каждого тайла и вывод в строку
  (bind _asthird_person_character (Utilities|Casting|CastToThirdPersonCharacter (Game|GetPlayerCharacter 0)))
  (Variables|/Script/Engine.CharacterMovementComponent|SetMaxWalkSpeed (Variables|/Script/Engine.Character|GetCharacterMovement _asthird_person_character) (Math|Float|Clamp(Float) (+ (Variables|/Script/Engine.CharacterMovementComponent|GetMaxWalkSpeed (Variables|/Script/Engine.Character|GetCharacterMovement _asthird_person_character)) 1.01) 6e+02 2e+03))
  (Development|PrintString (Utilities|String|ToString(Float) (Variables|/Script/Engine.CharacterMovementComponent|GetMaxWalkSpeed (Variables|/Script/Engine.Character|GetCharacterMovement _asthird_person_character))))
  ;[1 1 1] Destroy road behind
  (Utilities|FlowControl|Delay 2.0)
  (Actor|DestroyActor))

(event EventBeginPlay
  ;[1 0.335 0.195] Попытка отправить координаты для получения в другом блюпринте (ThirdPersonCharacter)
  (bind _output_get (Variables|Default|SetLineLocationX (Utilities|Array|MakeArray (.x (Transformation|GetWorldLocation (Variables|Default|GetLine4))) (.x (Transformation|GetWorldLocation (Variables|Default|GetLine3))) (.x (Transformation|GetWorldLocation (Variables|Default|GetLine2))) (.x (Transformation|GetWorldLocation (Variables|Default|GetLine1))))))
  (for _array_element _output_get
    (Development|PrintString (Utilities|String|ToString(Float) _array_element) true true "(R=1.000000,G=0.000000,B=0.008304,A=1.000000)" 5.0)))

(fn ConstructionScript)

(fn RandomSpawn
  ;[1 1 1] Заготовка для системы спавна на линии 1
  (if (Math|Float|InRange(Float) (Math|Random|RandomFloatinRange 0.0 1.0) 0.0 0.4)
    (Game|SpawnActorfromClass "/Game/CaRRunneR/BP/Spawn/BP_obstacle.BP_obstacle_C" (Transformation|GetWorldTransform (Variables|Default|GetLine1)) "Undefined" 0 0)))